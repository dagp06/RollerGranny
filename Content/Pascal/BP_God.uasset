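; BP_God is a gamepad-controlled spawner that drops obstacles into three lanes, apparently as a "god" role.
; The left, bottom and right face buttons each select an obstacle class (100t, Piano or Animal) and call SpawnObstacle with their lane number.
; SpawnObstacle spawns the current class at that lane's SpawnBox transform, looked up by GetLaneTransform.
; The left button's handler carries a "TO REMOVE" note.
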(event `self.ReceiveBeginPlay`
  (set `self.currentObject` "/Game/BP/FallingObjects/100t.100t_C"))

(event `Key|Gamepad_FaceButton_Left`
  (params (Key :type "Key Structure" :default "AnyKey"))
  (:`Pressed`
    ;[1 1 1] TO REMOVE
    (set `self.currentObject` "/Game/BP/FallingObjects/100t.100t_C")
    (`self.SpawnObstacle` 1)))

(event `Key|Gamepad_FaceButton_Bottom`
  (params (Key :type "Key Structure" :default "AnyKey"))
  (:`Pressed`
    ;[1 1 1] TO REMOVE
    (set `self.currentObject` "/Game/BP/FallingObjects/Piano.Piano_C")
    (`self.SpawnObstacle` 2)))

(event `Key|Gamepad_FaceButton_Right`
  (params (Key :type "Key Structure" :default "AnyKey"))
  (:`Pressed`
    ;[1 1 1] TO REMOVE
    (set `self.currentObject` "/Game/BP/FallingObjects/Animal.Animal_C")
    (`self.SpawnObstacle` 3)))

(fn `GetLaneTransform`
  (params (laneNumber :type Integer))
  (returns (NewParam :type "Transform Structure"))
  (switch `int` laneNumber
    (:`1`
      (return (`SceneComponent.K2_GetComponentToWorld` (`self.SpawnBox1`))))
    (:`2`
      (return (`SceneComponent.K2_GetComponentToWorld` (`self.SpawnBox2`))))
    (:`3`
      (return (`SceneComponent.K2_GetComponentToWorld` (`self.SpawnBox3`))))))

(fn `SpawnObstacle`
  (params (laneNumber :type Integer))
  (bind _newparam (`self.GetLaneTransform` laneNumber))
  (`|SpawnActorFromClass` (`self.currentObject`) _newparam "Undefined" "OverrideRootScale"))

(fn `UserConstructionScript`)