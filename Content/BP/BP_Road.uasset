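; BP_Road is an actor that maintains a rolling chain of BP_RoadSegment actors as a continuously extending road.
; On BeginPlay it registers the StartSegment child actor, then appends InitialLength segments, each spawned at the previous one's AttachPoint2 and attached to the road root.
; Tick calls Rotate each time DelayRotate elapses, which clears and destroys the oldest segment and spawns a new one at the end.
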(event EventBeginPlay
  (CallFunction|InitRoad))

(event EventActorBeginOverlap
  (params (OtherActor :type Actor%20Object%20Reference)))

(event EventTick
  (params (DeltaSeconds :type Float%20%28single-precision%29))
  (bind _output_get (Variables|Default|Settime (+ (Variables|Default|Gettime) DeltaSeconds)))
  (if (>= _output_get (Variables|Default|GetDelayRotate))
    (Variables|Default|Settime 0.0)
    (CallFunction|Rotate)))

(fn ConstructionScript)

(fn InitRoad
  (bind _asbp_road_segment (Utilities|Casting|CastToBP_RoadSegment (Variables|/Script/Engine.ChildActorComponent|GetChildActor (Variables|Default|GetStartSegment))))
  (Utilities|Array|Add (Variables|Default|GetRoadSegments) _asbp_road_segment)
  (for _index (range 0 (- (Variables|Default|GetInitialLength) 1))
    (CallFunction|AddNewSegment)))

(fn AddNewSegment
  (bind _roadsegments (Variables|Default|GetRoadSegments))
  (bind _returnvalue (Game|SpawnActorfromClass "/Game/BP/BP_RoadSegment.BP_RoadSegment_C" (Transformation|GetWorldTransform (Variables|/Game/BP/BP_RoadSegment.BP_RoadSegment_C|GetAttachPoint2 (Utilities|Array|Get(acopy) _roadsegments (Utilities|Array|LastIndex _roadsegments)))) "AlwaysSpawn" 0 0))
  (Utilities|Array|Add (Variables|Default|GetRoadSegments) _returnvalue)
  (Class|Actor|AttachRootComponentto _returnvalue (Variables|Default|GetDefaultSceneRoot) "None" "KeepWorldPosition" true))

(fn RemoveOldestSegment
  (bind _roadsegments (Variables|Default|GetRoadSegments))
  (bind _output_get (LocalVariables|Setdestroyed (Utilities|Array|Get(acopy) _roadsegments)))
  (Default|Clear _output_get)
  (Utilities|Array|RemoveItem _roadsegments _output_get)
  (Actor|DestroyActor _output_get))

(fn Rotate
  (CallFunction|RemoveOldestSegment)
  (CallFunction|AddNewSegment))