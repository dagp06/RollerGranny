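; BP_CatPlayground is a spawner actor that places BP_Obstacle_Cat obstacles relative to the moving player.
; SpawnCat gets the player through GM_Main and offsets the player mesh's X by X velocity times Distspeed, so placement scales with speed.
; Y, Z, rotation and scale come from the Arrow component; a zero Distspeed skips spawning.
; Nothing here calls SpawnCat, and debug prints remain.
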(event `self.ReceiveBeginPlay`)

(event `self.ReceiveActorBeginOverlap`
  (params (OtherActor :type "Actor Object Reference")))

(event `self.ReceiveTick`
  (params (DeltaSeconds :type "Float (single-precision)")))

(fn `SpawnCat`
  (bind _returnvalue (`SceneComponent.K2_GetComponentToWorld` (`self.Arrow`)))
  (bind _asgm_main (cast `/Game/BP/GM_Main` (`GameplayStatics.GetGameMode`)))
  (if (not (== (`self.distspeed`) 0.0))
    (bind _player (`/Game/BP/GM_Main.Player` _asgm_main))
    (bind _velocity_x (`KismetMathLibrary.BreakVector` (`MovementComponent.Velocity` (`/Game/ThirdPersonBP/Blueprints/SkaterDefaultPawn.FloatingPawnMovement` _player))))
    (bind _returnvalue_x (`KismetMathLibrary.BreakVector` (`SceneComponent.K2_GetComponentLocation` (`/Game/ThirdPersonBP/Blueprints/SkaterDefaultPawn.SkeletalMesh` _player))))
    (bind _returnvalue_2 (+ (* _velocity_x (`self.distspeed`)) _returnvalue_x))
    (`KismetSystemLibrary.PrintString` (`KismetStringLibrary.Conv_DoubleToString` _returnvalue_2))
    (`KismetSystemLibrary.PrintString` (`KismetStringLibrary.Conv_DoubleToString` _returnvalue_x))
    (`|SpawnActorFromClass` "/Game/BP/Obstacles/BP_Obstacle_Cat.BP_Obstacle_Cat_C" (`KismetMathLibrary.MakeTransform` (`KismetMathLibrary.MakeVector` _returnvalue_2 (.y (.location _returnvalue)) (.z (.location _returnvalue))) (.rotation _returnvalue) (.scale _returnvalue)) "AlwaysSpawn" "OverrideRootScale")))

(fn `UserConstructionScript`)